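; Treasure chest actor that ejects an inventory item when its SpawnItem event is called.
; The event spawns the configurable SpawnedClass at half scale just above the Chest component.
; If the result is a BP_BaseInventoryItem, it launches the item with a physics impulse on its Box, using the Vector variable.
; The graph contains no trigger or opening logic, and its Animation reference is unused.
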(event Custom|SpawnItem
  (bind _chest (Variables|Default|GetChest))
  (bind _returnvalue (Transformation|GetWorldLocation _chest))
  (bind (_x _y _z) (Math|Vector|BreakVector _returnvalue))
  (bind _returnvalue_2 (Game|SpawnActorfromClass (Variables|Default|GetSpawnedClass) (Math|Transform|MakeTransform (Math|Vector|MakeVector _x _y (+ _z 83.0)) "0,0.000000, 0" "0.500000,0.500000,0.500000") "Undefined" 0 0))
  (bind _asbp_base_inventory_item (Utilities|Casting|CastToBP_BaseInventoryItem _returnvalue_2))
  (Physics|AddImpulse (Variables|/Game/Megicka/Core/Inventory/BP_BaseInventoryItem.BP_BaseInventoryItem_C|GetBox _asbp_base_inventory_item) (Variables|Default|GetVector) "None" false))

(event Input|KeyboardEvents|6
  (params (Key :type Key%20Structure :default "None")))

(fn ConstructionScript)