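; Multiplayer game mode that carries each player's staff across map changes and hands out player starts.
; Before opening a map, it saves staff classes by player name in BP_GameInstance, then delegates travel there after a delay.
; After each login and a delay, it reapplies saved staffs to all controlled characters through a server event.
; Player starts are gathered at construction and removed as assigned, so each is used once.
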(event Custom|SaveStaffs
  ;[1 0.9157 0.4371 1 28] Save staffs
  (for _array_element (Variables|Default|GetAllPlayerControllers)
    (bind _asbp_main_character (Utilities|Casting|CastToBP_MainCharacter (Pawn|GetControlledPawn _array_element)))
    (Utilities|Map|Add (Variables|/Game/Megicka/Core/BP_GameInstance.BP_GameInstance_C|GetAllStaffForCharacters (Variables|Default|GetMainGameInstance)) (PlayerState|GetPlayerName (Variables|/Script/Engine.Controller|GetPlayerState _array_element)) (.AsBP%20Base%20Staff (Utilities|Casting|CastToBP_BaseStaffClass (Variables|/Script/Engine.ChildActorComponent|GetChildActorClass (Variables|/Game/Megicka/Core/Characters/BP_MainCharacter.BP_MainCharacter_C|GetStaff _asbp_main_character))))))
  (Utilities|PrintPlayerStaffLenght))

(event Custom|OpenMap
  (params (Map :type String))
  ;[0.972 1 0.5109 1 28] Event: Open Map
  (CallFunction|SaveStaffs)
  (Utilities|FlowControl|Delay 2.0)
  (Default|OpenMap (Variables|Default|GetMainGameInstance) Map))

(event EventPostLogin
  (params (NewPlayer :type Player%20Controller%20Object%20Reference))
  (Utilities|Array|Add (Variables|Default|GetAllPlayerControllers) NewPlayer)
  (Utilities|FlowControl|Delay 3.0)
  (for _array_element (Variables|Default|GetAllPlayerControllers)
    (Utilities|IsValid (Pawn|GetControlledPawn _array_element)
      (:Is%20Valid
        (bind _asbp_main_character (Utilities|Casting|CastToBP_MainCharacter (Pawn|GetControlledPawn _array_element)))
        (Default|RE:StaffCharServer _asbp_main_character (.Value (Utilities|Map|Find (Variables|/Game/Megicka/Core/BP_GameInstance.BP_GameInstance_C|GetAllStaffForCharacters (Variables|Default|GetMainGameInstance)) (PlayerState|GetPlayerName (Variables|/Script/Engine.Controller|GetPlayerState _array_element)))))))))

(event EventBeginPlay
  ;[1 0.4792 0.4792 1 28] BeginPlay
  ;;[1 1 1] Set Game Instance variable
  (bind _asbp_game_instance (Utilities|Casting|CastToBP_GameInstance (Game|GetGameInstance)))
  (Variables|Default|SetMainGameInstance _asbp_game_instance))

(event EventHandleStartingNewPlayer
  (params (NewPlayer :type Player%20Controller%20Object%20Reference))
  (|CallParentFunction NewPlayer))

(fn ConstructionScript
  (bind _outactors (Actor|GetAllActorsOfClass "/Script/Engine.PlayerStart"))
  (Variables|Default|SetPlayer%20Starts _outactors))

(fn ChoosePlayerStart
  (params (Player :type Controller%20Object%20Reference))
  (bind _player_starts (Variables|Default|GetPlayer%20Starts))
  (bind _output_get (Variables|Default|SetSelectedPlayerStart (Utilities|Array|Get(acopy) _player_starts)))
  (Utilities|Array|RemoveItem _player_starts _output_get)
  (return (Variables|Default|GetSelectedPlayerStart)))