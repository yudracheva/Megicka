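; Base staff weapon that fires a spawned actor, likely a projectile, from its Arrow component, with a reload cooldown.
; Shoot passes the Arrow's transform at reduced scale (marked as a workaround) through ShootServer to ShootMulti, a server-to-multicast chain judging by the names.
; ShootMulti gates on Reload, spawns the configured class with damage and X-offset values, then clears the flag after TimeReload.
; A separate function, not called here, assigns and activates the muzzle effect.
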(event Custom|Shoot
  (bind _arrow (Variables|Default|GetArrow))
  (bind _returnvalue (Transformation|GetWorldTransform _arrow))
  (bind (_location _rotation) (Math|Transform|BreakTransform _returnvalue))
  (CallFunction|ShootServer (Math|Transform|MakeTransform _location _rotation "0.200000,0.200000,0.200000")))

(event Custom|ShootServer
  (params (SpawnTransform :type Transform))
  (CallFunction|ShootMulti SpawnTransform))

(event Custom|ShootMulti
  (params (SpawnTransform :type Transform))
  (if (not (Variables|Default|GetReload))
    (Variables|Default|SetReload true)
    (Game|SpawnActorfromClass (Variables|Default|GetClass) SpawnTransform "AlwaysSpawn" 0 (Variables|Default|GetDamage) (Variables|Default|GetDelta%20Location%20X) 0)
    (Utilities|FlowControl|Delay (Variables|Default|GetTimeReload))
    (Variables|Default|SetReload false)))

(fn ConstructionScript)

(fn Muzzlefybc
  (bind _muzzle (Variables|VFX|GetMuzzle))
  (Class|NiagaraComponent|SetAsset _muzzle (Variables|VFX|GetMuzzleFX) true)
  (Components|Activation|SetActive _muzzle true false))