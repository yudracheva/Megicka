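; Base enemy that wanders, attacks a sighted main character from range, and dies when its HP runs out.
; A self-restarting AIMoveTo loop heads for random nearby points or the character spotted by PawnSensing, then turns and spawns an attack actor, even after a failed move.
; Damage updates the HP bar widget; death plays a sound, calls CallDead and destroys the actor after a delay.
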(event OnSeePawn(PawnSensing)
  (params (Pawn :type Pawn%20Object%20Reference))
  (bind _asbp_main_character (Utilities|Casting|CastToBP_MainCharacter Pawn))
  (if (not (Variables|/Game/Megicka/Core/Characters/MainCharacter/BP_MainCharacter.BP_MainCharacter_C|GetisDead _asbp_main_character))
    (Variables|Default|SetChar _asbp_main_character)
    (Variables|Default|SetAcceptance%20Radius 7e+02)))

(event Custom|Move
  (CallFunction|MoveServer))

(event Custom|MoveServer
  (CallFunction|MoveMulti))

(event Custom|MoveMulti
  (bind _scene (Variables|Default|GetScene))
  (bind _returnvalue (Transformation|GetWorldTransform _scene))
  (bind (_location _rotation) (Math|Transform|BreakTransform _returnvalue))
  (if (not (Variables|Default|GetisDead))
    (AI|AIMoveTo self (Math|Random|RandomPointinBoundingBox (Transformation|GetActorLocation) "700.000000,700.000000,100.000000") (Variables|Default|GetChar) (Variables|Default|GetAcceptance%20Radius) false
      (:OnSuccess
        _)
      (:OnFail
        _))
    (Utilities|FlowControl|Delay 1.0)
    (Utilities|IsValid (Variables|Default|GetChar)
      (:Is%20Valid
        (Transformation|SetActorRotation (Math|Rotator|MakeRotator 0.0 0.0 (.Yaw (Math|Rotator|BreakRotator (Math|Rotator|FindLookatRotation (Transformation|GetActorLocation) (Transformation|GetActorLocation (Variables|Default|GetChar)))))))
        (Variables|Attack|SetisAttack true)
        (Utilities|FlowControl|Delay (Variables|Attack|GetAttackDelay))
        (Audio|PlaySoundatLocation (Variables|Default|GetAttackSound) _location "0, 0, 0" 1.0 1.0 0.0 0 0 0)
        (Game|SpawnActorfromClass (Variables|Attack|GetClassAttack) (Math|Transform|MakeTransform _location _rotation "0.200000,0.200000,0.200000") "Undefined" 0 1e+01 3e+01 0)
        (Variables|Attack|SetisAttack false)
        (Utilities|FlowControl|Delay (Variables|Attack|GetDurationAfterAttack)))
      (:Is%20Not%20Valid
        _))
    (CallFunction|Move)))

(event Custom|UpdateHPMulti
  (params (Value :type Float%20%28single-precision%29))
  (Variables|/Game/Megicka/UI/UserInterface/WBP_HP.WBP_HP_C|SetValue (Variables|Default|GetAs%20WBP%20HP) Value))

(event EventBeginPlay
  (Variables|Default|SetHp (Variables|Default|GetMaxHP))
  (bind _aswbp_hp (Utilities|Casting|CastToWBP_HP (UserInterface|GetWidget (Variables|Default|GetHPBar))))
  (Variables|Default|SetAs%20WBP%20HP _aswbp_hp)
  (Variables|/Game/Megicka/UI/UserInterface/WBP_HP.WBP_HP_C|SetValue _aswbp_hp (Variables|Default|GetHp))
  (Variables|/Game/Megicka/UI/UserInterface/WBP_HP.WBP_HP_C|SetMaxValue _aswbp_hp (Variables|Default|GetMaxHP))
  (CallFunction|Move))

(event Game|Damage|EventAnyDamage
  (params (Damage :type Float%20%28single-precision%29) (DamageType :type Damage%20Type%20Object%20Reference) (InstigatedBy :type Controller%20Object%20Reference) (DamageCauser :type Actor%20Object%20Reference))
  (Class|BPITypeDamageInterface|DamageEvent(Message) DamageType (Variables|Default|GetDamageEventType))
  (bind _output_get (Variables|Default|SetHp (- (Variables|Default|GetHp) Damage)))
  (CallFunction|UpdateHPMulti _output_get)
  (if (<= _output_get 0.0)
    (if (not (Variables|Default|GetisDead))
      (Audio|PlaySoundatLocation (Variables|Default|GetDeathSound) (Transformation|GetWorldLocation (Variables|Character|GetMesh)) "0, 0, 0" 1.0 1.0 0.0 0 0 0)
      (Variables|Default|SetisDead true)
      (Default|CallDead)
      (Utilities|FlowControl|Delay 5.0)
      (Actor|DestroyActor))))

(fn ConstructionScript)