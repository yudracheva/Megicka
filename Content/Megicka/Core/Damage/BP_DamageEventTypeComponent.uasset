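; Actor component that gives its owner a visual or status effect actor matching the type of damage received.
; DamageEvent switches on the damage type (Water, Fire, Charge or River) and spawns the matching effect actor at the owner's transform.
; Each effect snaps onto the owner at the "Effect" socket; only the Charge energy effect also sets the owner as its Owner.
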(fn DamageEvent
  (params (DamageType :type EAllDamageType%20Enum :default "NewEnumerator0"))
  (bind _returnvalue (Components|GetOwner))
  (switch Utilities|FlowControl|Switch|SwitchonEAllDamageType DamageType
    (:NewEnumerator0
      (bind _returnvalue_2 (Game|SpawnActorfromClass "/Game/Megicka/Core/Damage/BP_EffectWater.BP_EffectWater_C" (Transformation|GetActorTransform (Components|GetOwner)) "Undefined" 0 0))
      (Transformation|AttachActorToActor _returnvalue_2 (Components|GetOwner) "Effect" "SnapToTarget" "SnapToTarget" "SnapToTarget" true))
    (:NewEnumerator1
      (bind _returnvalue_3 (Game|SpawnActorfromClass "/Game/Megicka/Core/Damage/BP_EffectFire.BP_EffectFire_C" (Transformation|GetActorTransform (Components|GetOwner)) "Undefined" 0 0))
      (Transformation|AttachActorToActor _returnvalue_3 (Components|GetOwner) "Effect" "SnapToTarget" "SnapToTarget" "SnapToTarget" true))
    (:NewEnumerator2
      (bind _returnvalue_4 (Game|SpawnActorfromClass "/Game/Megicka/Core/Damage/BP_EffectEnergy.BP_EffectEnergy_C" (Transformation|GetActorTransform _returnvalue) "Undefined" _returnvalue 0))
      (Transformation|AttachActorToActor _returnvalue_4 (Components|GetOwner) "Effect" "SnapToTarget" "SnapToTarget" "SnapToTarget" true))
    (:NewEnumerator3
      (bind _returnvalue_5 (Game|SpawnActorfromClass "/Game/Megicka/Core/Damage/BP_EffectRiver.BP_EffectRiver_C" (Transformation|GetActorTransform (Components|GetOwner)) "Undefined" 0 0))
      (Transformation|AttachActorToActor _returnvalue_5 (Components|GetOwner) "Effect" "SnapToTarget" "SnapToTarget" "SnapToTarget" true))))