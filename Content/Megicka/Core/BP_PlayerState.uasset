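; Player state Blueprint that stores each player's name, clothing color, staff color and inventory slots.
; Setters route through server events into multicast events that write the variables, with plain getters for reading them.
; CopyProperties, on authority, passes all four values to the new player state through those setters.
; The construction script defaults both colors to the "Blue" rows of the cloth and staff settings data tables.
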(event Custom|SaveStaffColorServer
  (params (Color :type String))
  ;[1 1 1] Save color variable
  (CallFunction|SaveStaffColorMulticast Color))

(event Custom|SaveStaffColorMulticast
  (params (Color :type String))
  ;[1 1 1] Save color variable
  (Variables|Default|SetStaff Color))

(event Custom|SaveNameVariableServer
  (params (Name :type String))
  ;[1 1 1] Save name variable
  (CallFunction|SaveNameVariableMulticast Name))

(event Custom|SaveNameVariableMulticast
  (params (Name :type String))
  ;[1 1 1] Save name variable
  (Variables|Default|SetName Name))

(event Custom|SaveColorVariableServer
  (params (Color :type String))
  ;[1 1 1] Save color variable
  (CallFunction|SaveColorVariableMulticast Color))

(event Custom|SaveColorVariableMulticast
  (params (Color :type String))
  ;[1 1 1] Save color variable
  (Variables|Default|SetColor Color))

(event Custom|saveInventorySer
  (params (InventorySlots :type Array%20of%20S%20Slot%20Structures))
  (CallFunction|SaveInventoryMulti InventorySlots))

(event Custom|SaveInventoryMulti
  (params (InventorySlots :type Array%20of%20S%20Slot%20Structures))
  (Variables|Default|SetInventorySlots InventorySlots))

(event EventCopyProperties
  (params (NewPlayerState :type Player%20State%20Object%20Reference))
  (Networking|SwitchHasAuthority
    (:Authority
      (bind _asbp_player_state (Utilities|Casting|CastToBP_PlayerState NewPlayerState))
      (CallFunction|SetName _asbp_player_state (Variables|Default|GetName))
      (CallFunction|SetColor _asbp_player_state (Variables|Default|GetColor))
      (CallFunction|SetStaffColor _asbp_player_state (Variables|Default|GetStaff))
      (CallFunction|SetInventorySlots _asbp_player_state (Variables|Default|GetInventorySlots)))))

(fn ConstructionScript
  (bind _returnvalue (Utilities|GetDataTableRow "/Game/Megicka/Core/Characters/MainCharacter/DT_CharacterClothsSettings.DT_CharacterClothsSettings" "Blue")
    (:then
      (Variables|Default|SetColor (.ColorName (Utilities|Struct|BreakFCharacterClothsStruct _returnvalue)))
      (bind _returnvalue_2 (Utilities|GetDataTableRow "/Game/Megicka/Core/Characters/MainCharacter/DT_CharacterStaffSettings.DT_CharacterStaffSettings" "Blue")
        (:then
          (Variables|Default|SetStaff (.ColorName (Utilities|Struct|BreakFStaffStruct _returnvalue_2))))))))

(fn GetName
  (return (Variables|Default|GetName)))

(fn SetName
  (params (Name :type String))
  (CallFunction|SaveNameVariableServer Name))

(fn GetColor
  (return (Variables|Default|GetColor)))

(fn SetColor
  (params (Color :type String))
  (CallFunction|SaveColorVariableServer Color))

(fn GetStaffColor
  (return (Variables|Default|GetStaff)))

(fn SetStaffColor
  (params (Staff :type String))
  (CallFunction|SaveStaffColorServer Staff))

(fn SetInventorySlots
  (params (InventorySlots :type Array%20of%20S%20Slot%20Structures))
  (CallFunction|SaveInventorySer InventorySlots))

(fn GetInventorySlots
  (return (Variables|Default|GetInventorySlots)))