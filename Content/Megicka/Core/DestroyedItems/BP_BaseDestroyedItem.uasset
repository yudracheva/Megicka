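; BP_BaseDestroyedItem is a base actor for destructible props that explode when shot.
; The construction script applies the configurable Mesh to the Cube component.
; A hit from an actor tagged "Bullet" calls DestroyObjectServer, which relays to DestroyObjectMulti, named as a server-to-multicast pair.
; That event spawns attached explosion particles and sound, clears the mesh, then destroys the actor after a short delay.
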(event OnComponentHit(Cube)
  (params (HitComponent :type Primitive%20Component%20Object%20Reference) (OtherActor :type Actor%20Object%20Reference) (OtherComp :type Primitive%20Component%20Object%20Reference) (NormalImpulse :type Vector :default "0, 0, 0") (Hit :type Hit%20Result%20Structure%20%28by%20ref%29))
  (if (Actor|ActorHasTag OtherActor "Bullet")
    (CallFunction|DestroyObjectServer)))

(event Custom|DestroyObjectServer
  (CallFunction|DestroyObjectMulti))

(event Custom|DestroyObjectMulti
  (bind _cube (Variables|Default|GetCube))
  (Effects|SpawnEmitterAttached "/Game/StarterContent/Particles/P_Explosion.P_Explosion" _cube "None")
  (Audio|SpawnSoundAttached "/Game/StarterContent/Audio/Explosion_Cue.Explosion_Cue" _cube "None" "0, 0, 0" "0, 0, 0" "KeepRelativeOffset" false 1.0 1.0 0.0 0 0)
  (Components|StaticMesh|SetStaticMesh (Variables|Default|GetCube) 0)
  (Utilities|FlowControl|Delay 2.0)
  (Actor|DestroyActor))

(event EventBeginPlay)

(event Collision|EventActorBeginOverlap
  (params (OtherActor :type Actor%20Object%20Reference)))

(event EventTick
  (params (DeltaSeconds :type Float%20%28single-precision%29)))

(fn ConstructionScript
  (Components|StaticMesh|SetStaticMesh (Variables|Default|GetCube) (Variables|Default|GetMesh)))