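; BP_SkeletonMage is a ranged enemy that roams until it sees the main character, then pursues and attacks it.
; A looping AIMoveTo heads to random nearby points until PawnSensing stores the player as target actor and widens the acceptance radius to casting range.
; After each move, successful or failed, it pauses, yaws toward any target and spawns a damaging actor at its Scene component.
; Incoming damage reduces Hp and destroys it at zero.
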(event OnSeePawn(PawnSensing)
  (params (Pawn :type Pawn%20Object%20Reference))
  (bind _asbp_main_character (Utilities|Casting|CastToBP_MainCharacter Pawn))
  (Variables|Default|SetChar _asbp_main_character)
  (Variables|Default|SetAcceptance%20Radius 7e+02))

(event Custom|Move
  (AI|AIMoveTo self (Math|Random|RandomPointinBoundingBox (Transformation|GetActorLocation) "700.000000,700.000000,100.000000") (Variables|Default|GetChar) (Variables|Default|GetAcceptance%20Radius) false
    (:OnSuccess
      _)
    (:OnFail
      _))
  (Utilities|FlowControl|Delay 1.0)
  (Utilities|IsValid (Variables|Default|GetChar)
    (:Is%20Valid
      (Transformation|SetActorRotation (Math|Rotator|MakeRotator 0.0 0.0 (.Yaw (Math|Rotator|BreakRotator (Math|Rotator|FindLookatRotation (Transformation|GetActorLocation) (Transformation|GetActorLocation (Variables|Default|GetChar)))))))
      (Game|SpawnActorfromClass (Variables|Default|GetClass) (Transformation|GetWorldTransform (Variables|Default|GetScene)) "Undefined" 0 1e+01 1e+01 0)
      (Utilities|FlowControl|Delay 1.0))
    (:Is%20Not%20Valid
      _))
  (CallFunction|Move))

(event EventBeginPlay
  (AI|AIMoveTo self (Math|Random|RandomPointinBoundingBox (Transformation|GetActorLocation) "700.000000,700.000000,100.000000") (Variables|Default|GetChar) (Variables|Default|GetAcceptance%20Radius) false
    (:OnSuccess
      _)
    (:OnFail
      _))
  (Utilities|FlowControl|Delay 1.0)
  (Utilities|IsValid (Variables|Default|GetChar)
    (:Is%20Valid
      (Transformation|SetActorRotation (Math|Rotator|MakeRotator 0.0 0.0 (.Yaw (Math|Rotator|BreakRotator (Math|Rotator|FindLookatRotation (Transformation|GetActorLocation) (Transformation|GetActorLocation (Variables|Default|GetChar)))))))
      (Game|SpawnActorfromClass (Variables|Default|GetClass) (Transformation|GetWorldTransform (Variables|Default|GetScene)) "Undefined" 0 1e+01 1e+01 0)
      (Utilities|FlowControl|Delay 1.0))
    (:Is%20Not%20Valid
      _))
  (CallFunction|Move))

(event Collision|EventActorBeginOverlap
  (params (OtherActor :type Actor%20Object%20Reference)))

(event EventTick
  (params (DeltaSeconds :type Float%20%28single-precision%29)))

(event Game|Damage|EventAnyDamage
  (params (Damage :type Float%20%28single-precision%29) (DamageType :type Damage%20Type%20Object%20Reference) (InstigatedBy :type Controller%20Object%20Reference) (DamageCauser :type Actor%20Object%20Reference))
  (Class|BPITypeDamageInterface|DamageEvent(Message) DamageType (Variables|Default|GetDAmageEventType))
  (bind _output_get (Variables|Default|SetHp (- (Variables|Default|GetHp) Damage)))
  (if (<= _output_get 0.0)
    (Actor|DestroyActor)))

(fn ConstructionScript)